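; BP_Item is a pickup actor for the inventory system that removes itself from the world when collected.
; When BP_player overlaps its Trigger, it plays a sound at the world origin and calls DestroyItem, which destroys the actor after a short delay.
; A separate PickUpItem function prints a message, calls the same DestroyItem and returns the Item value; the overlap path does not call it.
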(event `Destroy Item`
  (`KismetSystemLibrary.Delay` 0.1)
  (`self.K2_DestroyActor`))

(event `self.Trigger.OnComponentBeginOverlap`
  (params (OverlappedComponent :type "PrimitiveComponent Object Reference") (OtherActor :type "Actor Object Reference") (OtherComp :type "PrimitiveComponent Object Reference") (OtherBodyIndex :type Integer) (bFromSweep :type Boolean) (SweepResult :type "HitResult Structure (by ref)"))
  (cast `/Game/TopDown/Blueprints/BP_player` OtherActor)
  (`GameplayStatics.PlaySoundAtLocation` null (0.0 0.0 0.0) (struct) 1.0 1.0 0.0 null null null null)
  (`self.Destroy Item`))

(fn `Pick Up Item`
  (returns (Item :type String))
  (`KismetSystemLibrary.PrintString` "Item Picked")
  (`self.Destroy Item`)
  (return (`self.Item`)))

(fn `UserConstructionScript`)